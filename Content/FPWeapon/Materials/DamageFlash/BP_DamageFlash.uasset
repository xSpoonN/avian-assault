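; Actor component that briefly flashes its owner's skeletal mesh with an emissive color when the owner takes damage.
; On BeginPlay it binds to the owner's OnTakeAnyDamage and creates dynamic material instances for every slot of the first skeletal mesh found.
; Each hit sets their emissive color and multiplier from the flash settings, then zeroes both after a Delay of Duration, regardless of damage amount.
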(event Custom|DamageFlash
  (params (DamagedActor :type Actor%20Object%20Reference) (Damage :type Float%20%28single-precision%29) (DamageType :type Damage%20Type%20Object%20Reference) (InstigatedBy :type Controller%20Object%20Reference) (DamageCauser :type Actor%20Object%20Reference))
  (for _array_element (Variables|Default|GetFlashMaterials)
    (Rendering|Material|SetVectorParameterValue _array_element "EmissiveColor" (Variables|Default|GetFlashColor) :!class /Script/Engine.MaterialInstanceDynamic)
    (Rendering|Material|SetScalarParameterValue _array_element "EmissiveMultiplier" (Variables|Default|GetFlashIntensity) :!class /Script/Engine.MaterialInstanceDynamic))
  (Utilities|FlowControl|Delay (Variables|Default|GetDuration))
  (for _array_element_2 (Variables|Default|GetFlashMaterials)
    (Rendering|Material|SetVectorParameterValue _array_element_2 "EmissiveColor" "(R=0.000000,G=0.000000,B=0.000000,A=0.000000)" :!class /Script/Engine.MaterialInstanceDynamic)
    (Rendering|Material|SetScalarParameterValue _array_element_2 "EmissiveMultiplier" 0.0 :!class /Script/Engine.MaterialInstanceDynamic)))

(event EventBeginPlay
  (bind _output_get (Variables|Default|SetOwner (Components|GetOwner)))
  (EventDispatchers|BindEventtoOnTakeAnyDamage _output_get (EventDispatchers|CreateEvent :!event Custom|DamageFlash))
  ;[1 1 1] Create Dynamic Material
  (Utilities|IsValid (Actor|GetComponentbyClass (Variables|Default|GetOwner) "/Script/Engine.SkeletalMeshComponent")
    (:Is%20Valid
      (for (_array_element _array_index) (Rendering|Material|GetMaterials (Actor|GetComponentbyClass (Variables|Default|GetOwner) "/Script/Engine.SkeletalMeshComponent"))
        (bind _returnvalue (Rendering|Material|CreateDynamicMaterialInstance (Actor|GetComponentbyClass (Variables|Default|GetOwner) "/Script/Engine.SkeletalMeshComponent") _array_index _array_element "None" :!class /Script/Engine.PrimitiveComponent))
        (Utilities|Array|Add (Variables|Default|GetFlashMaterials) _returnvalue)))))