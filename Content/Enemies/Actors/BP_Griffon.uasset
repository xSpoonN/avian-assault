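; BP_Griffon is a griffon enemy Blueprint, currently set up as a test of volume-based pathfinding.
; On BeginPlay it finds a BP_CPathVolume in the level and asynchronously requests a path from its location to a hardcoded point.
; Success draws the debug path and prints a message, while failure prints the reason.
; It never follows the path, and the node that would run BT_AI_Flying is disconnected.
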(event EventBeginPlay
  (bind _returnvalue (Actor|GetActorOfClass "/CPathfinding/Blueprints/BP_CPathVolume.BP_CPathVolume_C"))
  (bind _output_get (Variables|Default|SetCPathVolume _returnvalue))
  (bind (_path _failreason) (|FindPathAsync _output_get (Transformation|GetActorLocation self) "0.000000,0.000000,600.000000" 2 0 0.2)
    (:Success
      (Class|CPathVolume|DrawDebugPath (Variables|Default|GetCPathVolume) _path 0.0 true "(B=255,G=0,R=255,A=255)")
      (Development|PrintString "Success!!"))
    (:Failure
      (Development|PrintString (Utilities|String|EnumtoString _failreason)))))

(event Collision|EventActorBeginOverlap
  (params (OtherActor :type Actor%20Object%20Reference)))

(event EventTick
  (params (DeltaSeconds :type Float%20%28single-precision%29)))

(fn ConstructionScript)