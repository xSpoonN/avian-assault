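; BP_Enemy is an enemy with health that dies once, as a ragdolling griffon that notifies the game state to check for the end.
; Death stops AI logic, plays the animation and delays destruction, much more briefly when the player's Powerup3 is active.
; With that powerup, destruction spawns an explosion that sphere-traces nearby pawns and damages each unique enemy, so kills can chain.
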(event Custom|Die
  (Physics|SetSimulatePhysics (Variables|Character|GetMesh) true)
  (AI|Logic|StopLogic (Variables|/Script/AIModule.AIController|GetBrainComponent (AI|GetAIController self)) "")
  (Components|Animation|PlayAnimation (Variables|Character|GetMesh) "/Game/QuadrapedCreatures/Griffon/Animations/ANIM_Griffon_Death.ANIM_Griffon_Death" false)
  (Default|CheckEnd (.AsBP%20AA%20Game%20State (Utilities|Casting|CastToBP_AA_GameState (Game|GetGameState))))
  (Utilities|FlowControl|Delay (Math|Float|SelectFloat 0.6 1e+01 (Variables|/Game/FirstPerson/Blueprints/BP_FirstPersonCharacter.BP_FirstPersonCharacter_C|GetPowerup3Active (.AsBP%20First%20Person%20Character (Utilities|Casting|CastToBP_FirstPersonCharacter (Game|GetPlayerCharacter 0))))))
  (Actor|DestroyActor))

(event Custom|Damage
  (params (DamageAmount :type Float%20%28double-precision%29))
  (bind _output_get (Variables|Default|SetHealth (- (Variables|Default|GetHealth) DamageAmount)))
  (if (<= _output_get 0.0)
    (if (not (Variables|Default|GetDead))
      (Variables|Default|SetDead true)
      (CallFunction|Die))))

(event EventDestroyed
  (bind _returnvalue (Transformation|GetActorLocation))
  (if (Variables|/Game/FirstPerson/Blueprints/BP_FirstPersonCharacter.BP_FirstPersonCharacter_C|GetPowerup3Active (.AsBP%20First%20Person%20Character (Utilities|Casting|CastToBP_FirstPersonCharacter (Game|GetPlayerCharacter 0))))
    (bind _outhits (Collision|MultiSphereTraceForObjects _returnvalue _returnvalue 1e+03 (Utilities|Array|MakeArray "ObjectTypeQuery3") false 0 "None"))
    (Effects|SpawnEmitteratLocation "/Game/MilitaryWeapDark/FX/P_Explosive_Rounds.P_Explosive_Rounds" _returnvalue "0, 0, 0" "5.000000,5.000000,5.000000")
    (Audio|SpawnSoundatLocation "/Game/MilitaryWeapDark/Sound/GrenadeLauncher/GrenadeLauncher_Explosion_Cue.GrenadeLauncher_Explosion_Cue" _returnvalue "0, 0, 0" 0.5 1.0 0.0 0 0)
    (for _array_element _outhits
      (Utilities|Set|Add (Variables|Default|GetDamageSet) (.HitActor (Collision|BreakHitResult _array_element))))
    (bind _result (Utilities|Set|ToArray (Variables|Default|GetDamageSet)))
    (for _array_element_2 _result
      (bind _asbp_enemy (Utilities|Casting|CastToBP_Enemy _array_element_2))
      (CallFunction|Damage _asbp_enemy 4e+01))
    (Actor|DestroyActor)
    (else
      (Actor|DestroyActor))))

(fn ConstructionScript)