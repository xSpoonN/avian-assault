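; BP_EnemySpawner periodically spawns enemies around its location, up to the round's enemy limit.
; A looping timer with a randomized initial delay fires SpawnEnemy, which, while Active, spawns up to Multiplier actors of the configured Class at random 3D offsets.
; Each spawn checks and increments the shared counter in BP_AA_GameState and prints a debug message.
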(event Custom|SpawnEnemy
  (bind _returnvalue (Game|GetGameState))
  (bind _asbp_aa_game_state (Utilities|Casting|CastToBP_AA_GameState _returnvalue))
  (if (Variables|Default|GetActive)
    (for _index (range 1 (Variables|Default|GetMultiplier))
      (if (< (Variables|/Game/FirstPerson/Blueprints/BP_AA_GameState.BP_AA_GameState_C|GetEnemiesSpawned _asbp_aa_game_state) (Variables|/Game/FirstPerson/Blueprints/BP_AA_GameState.BP_AA_GameState_C|GetEnemiesThisRound _asbp_aa_game_state))
        (Game|SpawnActorfromClass (Variables|Default|GetClass) (Math|Conversions|ToTransform(Vector) (+ (Transformation|GetActorLocation) (Math|Vector|MakeVector (Math|Random|RandomFloatinRange -5e+02 5e+02) (Math|Random|RandomFloatinRange -5e+02 5e+02) (Math|Random|RandomFloatinRange -5e+02 5e+02)))) "AdjustIfPossibleButAlwaysSpawn" "MultiplyWithRoot" 0 0)
        (Math|Integer|IncrementInt (Variables|/Game/FirstPerson/Blueprints/BP_AA_GameState.BP_AA_GameState_C|GetEnemiesSpawned (.AsBP%20AA%20Game%20State (Utilities|Casting|CastToBP_AA_GameState (Game|GetGameState))))
          (:%20%20
            (Development|PrintString "SPAWN" true true "(R=1.000000,G=0.000000,B=0.938498,A=1.000000)")))))))

(event EventBeginPlay
  (Utilities|Time|SetTimerbyEvent (delegate Custom|SpawnEnemy) (Variables|Default|GetTimeInterval) true 1.0 1e+01))

(fn ConstructionScript)